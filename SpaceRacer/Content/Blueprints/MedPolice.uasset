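; MedPolice is an actor, apparently a police enemy, that automatically fires Laser actors along its up vector.
; BeginPlay fires once and starts a looping timer that repeats FireShot, which spawns a Laser ahead with sound and debug prints.
; Hit applies point damage and destroys the actor, but the Laser cast supplying the damage causer is unwired.
; FireShot's fire-rate timer names an expiry function absent from this file.
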(event Custom|Printer
  (Development|PrintString "Hello" true true "(R=1.000000,G=0.851686,B=0.055066,A=1.000000)")
  (CallFunction|FireShot))

(event Collision|EventHit
  (params (MyComp :type Primitive%20Component%20Object%20Reference) (Other :type Actor%20Object%20Reference) (OtherComp :type Primitive%20Component%20Object%20Reference) (bSelfMoved :type Boolean) (HitLocation :type Vector :default "0, 0, 0") (HitNormal :type Vector :default "0, 0, 0") (NormalImpulse :type Vector :default "0, 0, 0") (Hit :type Hit%20Result%20Structure%20%28by%20ref%29))
  (Game|Damage|ApplyPointDamage 0 1.0 HitNormal Hit 0 (stale _aslaser))
  (Actor|DestroyActor))

(event EventBeginPlay
  (Utilities|Time|SetTimerbyEvent (delegate Custom|Printer) 0.5 true)
  (CallFunction|FireShot))

(fn ConstructionScript)

(fn FireShot
  (bind _returnvalue (Transformation|GetActorUpVector))
  (bind _returnvalue_2 (Transformation|GetActorLocation))
  (bind _returnvalue_3 (* _returnvalue 1e+03))
  (bind _returnvalue_4 (+ _returnvalue_2 _returnvalue_3))
  (Development|PrintString (Utilities|String|ToString(Vector) _returnvalue_4) true true "(R=1.000000,G=0.000000,B=0.236117,A=1.000000)")
  (Game|SpawnActorfromClass "/Game/Blueprints/Laser.Laser_C" (Math|Transform|MakeTransform _returnvalue_4 (Math|Rotator|FindLookatRotation _returnvalue_2 _returnvalue_4)) true 0 0)
  (Audio|PlaySoundatLocation 0 _returnvalue_4)
  (Variables|Default|SetCanFire true)
  (Utilities|Time|SetTimerbyFunctionName 0 "Shot Timer EXpired" (Variables|Default|GetFireRate)))